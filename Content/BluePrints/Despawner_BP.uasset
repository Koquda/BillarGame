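; Trigger actor for a billiards-style game that handles potted balls and players entering it.
; On overlap, casts sort the ball: the cue ball respawns at a set location, and the 8-ball runs its game-over check after a delay before being destroyed.
; Other balls are destroyed, then increment the Partida game mode's potted count with a coin sound.
; An overlapping Jugador plays a falling sound and returns to the main menu.
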(event `self.ReceiveActorBeginOverlap`
  (params (OtherActor :type "Actor Object Reference"))
  ;[1 1 1] Que pasa si una bola es entronada
  (`|ExecutionSequence`
    (:`then_0`
      (bind _asbola_bp (cast `/Game/BluePrints/Bolas/Bola_BP` OtherActor))
      (bind _asbola_blanca (cast `/Game/BluePrints/Bolas/Bola_Blanca` _asbola_bp)
        (:`then`
          (`self.K2_DestroyActor` _asbola_blanca)
          (`|SpawnActorFromClass` "/Game/BluePrints/Bolas/Bola_Blanca.Bola_Blanca_C" (`KismetMathLibrary.MakeTransform` (`self.SpawnBolaBlanca`)) "Undefined" "OverrideRootScale" null null))
        (:`CastFailed`
          (bind _asbola_8 (cast `/Game/BluePrints/Bolas/Bola8` _asbola_bp)
            (:`then`
              (`KismetSystemLibrary.Delay` 1.0)
              (`/Game/BluePrints/Bolas/Bola8.CheckGameDone` _asbola_8)
              (`self.K2_DestroyActor` _asbola_bp))
            (:`CastFailed`
              (`self.K2_DestroyActor` _asbola_bp)
              (`KismetSystemLibrary.Delay` 1.0)
              (bind _aspartida (cast `/Game/ModosDeJuego/Partida` (`GameplayStatics.GetGameMode`)))
              (`/Game/ModosDeJuego/Partida.IncrementarBolasEntronadas` _aspartida 1)
              (`GameplayStatics.PlaySound2D` "/Game/Audio/Coins_10.Coins_10" 1.0 1.0 0.0 null null))))))
    (:`then_1`
      (cast `/Game/BluePrints/Jugador/Jugador` OtherActor)
      (`GameplayStatics.PlaySound2D` "/Game/Audio/Cartoon_Falling_03.Cartoon_Falling_03" 1.0 1.0 0.0 null null)
      (`GameplayStatics.OpenLevel` "MainMenu"))))

(fn `UserConstructionScript`)