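; Bola_Blanca is the white ball, an actor that the player character can hit.
; On overlap with a Jugador it registers itself in that player's Bola reference, and clears it when the overlap ends.
; The BolaHit event launches the ball's Sphere with a very large impulse along the forward vector of player character 0.
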(event `self.ReceiveActorBeginOverlap`
  (params (OtherActor :type "Actor Object Reference"))
  ;[1 1 1] Settear la bola blanca como overlapping
  (bind _asjugador (cast `/Game/BluePrints/Jugador/Jugador` OtherActor))
  (set `/Game/BluePrints/Jugador/Jugador.Bola` self _asjugador))

(event `self.ReceiveActorEndOverlap`
  (params (OtherActor :type "Actor Object Reference"))
  ;[1 1 1] Settear la bola blanca como overlapping
  (bind _asjugador (cast `/Game/BluePrints/Jugador/Jugador` OtherActor))
  (set `/Game/BluePrints/Jugador/Jugador.Bola` null _asjugador))

(event `BolaHit`
  ;[1 1 1] golpe a bola blanca
  (`PrimitiveComponent.AddImpulse` (`self.Sphere`) (* (`self.GetActorForwardVector` (`GameplayStatics.GetPlayerCharacter` 0)) 500000000.0) "None" false))

(fn `UserConstructionScript`
  (`parent.UserConstructionScript`))