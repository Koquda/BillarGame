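; Bola8 is the black eight ball of a billiards game, handling the end-of-game check for when it is pocketed.
; CheckGameDone casts the game mode to Partida and compares its BolasEntronadas count with PuntosParaGanar, printing a win or loss message.
; Both outcomes open MainMenu; the author marks the logic unfinished, and nothing in this Blueprint calls the event.
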(event `CheckGameDone`
  ;[1 1 1] Comprobacion de fin de juego al entronar la bola negra (QUEDA TERMINARLO)
  (bind _aspartida (cast `/Game/ModosDeJuego/Partida` (`GameplayStatics.GetGameMode`)))
  (if (== (`/Game/ModosDeJuego/Partida.BolasEntronadas` _aspartida) (`self.Puntos para ganar`))
    (`KismetSystemLibrary.PrintString` "Ganaste")
    (`GameplayStatics.OpenLevel` "MainMenu")
    (else
      (`KismetSystemLibrary.PrintString` "Perdiste")
      (`GameplayStatics.OpenLevel` "MainMenu"))))

(fn `UserConstructionScript`
  (`parent.UserConstructionScript`))